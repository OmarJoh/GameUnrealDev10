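; Interactable chest Blueprint that opens its lid and notifies a linked key that the chest is open.
; The FInteract event plays a Timeline that rotates the lid toward 90 degrees, casting the Key reference to BP_Key1 and setting its ChestOpen flag on each update.
; A sphere overlap shows or hides a widget as an actor tagged Player enters or leaves.
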(event OnComponentBeginOverlap(Sphere)
  (params (OverlappedComponent :type Primitive%20Component%20Object%20Reference) (OtherActor :type Actor%20Object%20Reference) (OtherComp :type Primitive%20Component%20Object%20Reference) (OtherBodyIndex :type Integer) (bFromSweep :type Boolean) (SweepResult :type Hit%20Result%20Structure%20%28by%20ref%29))
  (if (Actor|ActorHasTag (stale OnComponentEndOverlap(Sphere) OtherActor) "Player")
    (Rendering|SetVisibility (Variables|Default|GetWidget) true false)))

(event OnComponentEndOverlap(Sphere)
  (params (OverlappedComponent :type Primitive%20Component%20Object%20Reference) (OtherActor :type Actor%20Object%20Reference) (OtherComp :type Primitive%20Component%20Object%20Reference) (OtherBodyIndex :type Integer))
  (if (Actor|ActorHasTag OtherActor "Player")
    (Rendering|SetVisibility (Variables|Default|GetWidget) false false)))

(event EventBeginPlay)

(event Collision|EventActorBeginOverlap
  (params (OtherActor :type Actor%20Object%20Reference)))

(event EventTick
  (params (DeltaSeconds :type Float%20%28single-precision%29)))

(event EventFInteract
  (bind _newtrack_1 (Timeline|Timeline Play)
    (:Update
      (Transformation|SetRelativeRotation (Variables|Default|GetChest_Lid) (Math|Rotator|Lerp(Rotator) "0, 0, 0" "0.000000,0.000000,90.000000" _newtrack_1) false false)
      (bind _asbp_key_1 (Utilities|Casting|CastToBP_Key1 (Variables|Default|GetKey)))
      (Variables|/Game/BluePrint/Chest/BP_Key1.BP_Key1_C|SetChestOpen _asbp_key_1 true))))

(fn ConstructionScript)